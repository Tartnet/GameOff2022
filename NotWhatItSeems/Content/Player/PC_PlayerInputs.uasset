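; Player controller component or controller Blueprint that receives the player's movement, look and jump inputs.
; On BeginPlay it caches the BP_Player actor as PlayerRef.
; Movement and mouse-look axis inputs are forwarded through Call functions, apparently event dispatchers that the player's movement events bind to.
; Jump presses and releases call Jump and StopJumping directly on the cached player.
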(event EventBeginPlay
  (bind _returnvalue (Actor|GetActorOfClass "/Game/Player/BP_Player.BP_Player_C"))
  (Variables|Default|SetPlayerRef _returnvalue))

(event Input|ActionEvents|InputActionJump
  (params (Key :type Key%20Structure :default "None"))
  (bind _playerref (Variables|Default|GetPlayerRef))
  ;[1 1 1] Calls movement components that the player movement events are bound to
  (:Pressed
    (Character|Jump _playerref))
  (:Released
    (Character|StopJumping _playerref)))

(event Input|AxisEvents|InputAxisMoveForward/Back
  (params (AxisValue :type Float%20%28single-precision%29))
  ;[1 1 1] Calls movement components that the player movement events are bound to
  (Default|CallMoveForward/Back AxisValue))

(event Input|AxisEvents|InputAxisMoveRight/Left
  (params (AxisValue :type Float%20%28single-precision%29))
  ;[1 1 1] Calls movement components that the player movement events are bound to
  (Default|CallMoveRight/Left AxisValue))

(event Input|AxisEvents|InputAxisTurnRight/LeftMouse
  (params (AxisValue :type Float%20%28single-precision%29))
  ;[1 1 1] Calls movement components that the player movement events are bound to
  (Default|CallTurnRight/LeftMouse AxisValue))

(event Input|AxisEvents|InputAxisLookUp/DownMouse
  (params (AxisValue :type Float%20%28single-precision%29))
  ;[1 1 1] Calls movement components that the player movement events are bound to
  (Default|CallLookUp/DownMouse AxisValue))

(fn ConstructionScript)