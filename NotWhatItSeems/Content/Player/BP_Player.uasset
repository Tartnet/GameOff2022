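; BP_Player is the player character Blueprint, handling first-person style movement and mouse look.
; On BeginPlay it casts the player controller to PC_PlayerInputs and binds its own handlers to that controller's axis events.
; Movement follows the actor's forward and right vectors, while horizontal mouse input adds controller yaw.
; Vertical look bypasses controller pitch, accumulating a clamped YRotation applied as the Camera's relative pitch.
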(event Custom|YAxisMovement
  (params (RecievedAxis :type Float%20%28double-precision%29))
  (Pawn|Input|AddMovementInput (Transformation|GetActorForwardVector) RecievedAxis false))

(event Custom|XAxisMovement
  (params (RecievedAxis :type Float%20%28double-precision%29))
  (Pawn|Input|AddMovementInput (Transformation|GetActorRightVector) RecievedAxis false))

(event Custom|XAxisTurning
  (params (RecievedAxis :type Float%20%28double-precision%29))
  (Pawn|Input|AddControllerYawInput RecievedAxis))

(event Custom|YAxisTurning
  (params (RecievedAxis :type Float%20%28double-precision%29))
  (Transformation|SetRelativeRotation (Variables|Default|GetCamera) (Math|Rotator|MakeRotator 0.0 (Math|Float|Clamp(Float) (+ RecievedAxis (Variables|Default|GetYRotation)) -65.0 9e+01) 0.0) false false)
  (Variables|Default|SetYRotation (Math|Float|Clamp(Float) (+ RecievedAxis (Variables|Default|GetYRotation)) -65.0 9e+01)))

(event EventBeginPlay
  (bind _aspc_player_inputs (Utilities|Casting|CastToPC_PlayerInputs (Game|GetPlayerController 0)))
  (bind _output_get (Variables|Default|SetPlayerController _aspc_player_inputs))
  (EventDispatchers|BindEventtoMoveForward/Back _output_get (delegate Custom|YAxisMovement))
  (EventDispatchers|BindEventtoMoveRight/Left _output_get (delegate Custom|XAxisMovement))
  (EventDispatchers|BindEventtoTurnRight/LeftMouse _output_get (delegate Custom|XAxisTurning))
  (EventDispatchers|BindEventtoLookUp/DownMouse _output_get (delegate Custom|YAxisTurning)))

(fn ConstructionScript)